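; ResourceDrop is a pickup-style actor that pops upward with a physics impulse when spawned.
; While alive, its Cube spins around yaw at a configurable Speed and bobs vertically using a sine of game time.
; Destroying it plays a 2D Pop sound.
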(event `self.ReceiveTick`
  (params (DeltaSeconds :type "Float (single-precision)"))
  (bind _cube (`self.Cube`))
  (`SceneComponent.K2_AddLocalRotation` _cube (`KismetMathLibrary.MakeRotator` 0.0 0.0 (* DeltaSeconds (`self.Speed`))) false false)
  (`SceneComponent.K2_AddLocalOffset` _cube (`KismetMathLibrary.MakeVector` 0.0 0.0 (`KismetMathLibrary.Sin` (* (`KismetSystemLibrary.GetGameTimeInSeconds`) 2.0))) false false))

(event `self.ReceiveDestroyed`
  (`GameplayStatics.PlaySound2D` "/Game/Sounds/pop.pop"))

(event `self.ReceiveBeginPlay`
  (`PrimitiveComponent.AddImpulse` (`self.Base`) (0.0 0.0 2000.0) "None" false))

(fn `UserConstructionScript`)