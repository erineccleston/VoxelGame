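; Inventory component that stores items by name in a resizable set of stacking slots.
; Parallel Inventory and Quantity arrays are sized to StartingCapacity on BeginPlay, with "None" marking an empty slot.
; Add increments only the first matching stack below StackSize, otherwise fills the first empty slot or returns false.
; Remove decrements a slot and clears it at the last item, while Dump prints both arrays for debugging.
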(event `self.ReceiveBeginPlay`
  (bind _startingcapacity (`self.StartingCapacity`))
  (`KismetArrayLibrary.Array_Resize` (`self.Inventory`) _startingcapacity)
  (`KismetArrayLibrary.Array_Resize` (`self.Quantity`) _startingcapacity))

(event `Dump`
  (for (_array_element _array_index) (`self.Inventory`)
    (`KismetSystemLibrary.PrintString` (`KismetStringLibrary.Concat_StrStr` "Element " (`KismetStringLibrary.Conv_NameToString` _array_element) " Index " (`KismetStringLibrary.Conv_IntToString` _array_index))))
  (for (_array_element_2 _array_index_2) (`self.Quantity`)
    (`KismetSystemLibrary.PrintString` (`KismetStringLibrary.Concat_StrStr` "Element " (`KismetStringLibrary.Conv_IntToString` _array_element_2) " Index " (`KismetStringLibrary.Conv_IntToString` _array_index_2)))))

(fn `Add`
  (params (Name :type Name))
  (returns (Success :type Boolean))
  (locals (Index :type Integer))
  (bind _returnvalue (`KismetArrayLibrary.Array_Find` (`self.Inventory`)))
  (bind _output_get (set `local.Index` (`KismetArrayLibrary.Array_Find` (`self.Inventory`) Name)))
  (if (> _output_get -1)
    (bind _output (`|GetArrayItem` (`self.Quantity`) _output_get))
    (if (< _output (`self.StackSize`))
      (`/Engine/EditorBlueprintResources/StandardMacros.IncrementInt` _output
        (:`  `
          _))
      (else
        (if (> _returnvalue -1) :!label _label
          (bind _output_get_2 (set `local.Index` _returnvalue))
          (`KismetArrayLibrary.Array_Set` (`self.Inventory`) _output_get_2 Name)
          (`KismetArrayLibrary.Array_Set` (`self.Quantity`) _output_get_2 1)
          (else
            (return false)))))
    (else
      (goto _label)))
  (return true))

(fn `ClearSlot`
  (params (Index :type Integer))
  (`KismetArrayLibrary.Array_Set` (`self.Inventory`) Index)
  (`KismetArrayLibrary.Array_Set` (`self.Quantity`) Index))

(fn `GetCapacity`
  (returns (Capacity :type Integer))
  (return (`KismetArrayLibrary.Array_Length` (`self.Inventory`))))

(fn `GetInventory`
  (returns (Inventory :type "Array of Name") (Quantity :type "Array of Integer"))
  (return (`self.Inventory`) (`self.Quantity`)))

(fn `Remove`
  (params (Index :type Integer))
  (bind _output (`|GetArrayItem` (`self.Quantity`) Index))
  (if (> _output 1)
    (`/Engine/EditorBlueprintResources/StandardMacros.DecrementInt` _output)
    (else
      (`self.ClearSlot` Index))))

(fn `SetCapacity`
  (params (Capacity :type Integer))
  (`KismetArrayLibrary.Array_Resize` (`self.Inventory`) Capacity)
  (`KismetArrayLibrary.Array_Resize` (`self.Quantity`) Capacity))