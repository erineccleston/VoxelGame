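; MapGenerator is a Blueprint that builds a noise-based voxel map when play begins.
; It seeds simplex noise, samples it over a square grid, and spawns a VoxelBase_BP wherever the value clears a threshold, leaving gaps elsewhere.
; The grid lies in the vertical YZ plane, and each voxel receives its noise value as debug text.
; A disconnected branch that would call DebugInvis on low-noise voxels never runs.
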(event `self.ReceiveBeginPlay`
  (`SimplexNoiseBPLibrary.setNoiseSeed` (`self.Seed`))
  (for _index (range 50)
    (for _index_2 (range 50)
      (bind _returnvalue (`KismetMathLibrary.Conv_IntToDouble` _index))
      (bind _returnvalue_2 (`KismetMathLibrary.Conv_IntToDouble` _index_2))
      (bind _returnvalue_3 (`SimplexNoiseBPLibrary.SimplexNoise2D` (/ _returnvalue 20.0) (/ _returnvalue_2 20.0)))
      (if (> _returnvalue_3 -0.25)
        (bind _returnvalue_4 (`|SpawnActorFromClass` "/Game/Blueprints/Voxels/VoxelBase_BP.VoxelBase_BP_C" (`KismetMathLibrary.MakeTransform` (`KismetMathLibrary.MakeVector` 0.0 (* _returnvalue 100.0) (* _returnvalue_2 100.0))) "AlwaysSpawn" "OverrideRootScale" null (`KismetTextLibrary.Conv_DoubleToText` _returnvalue_3 "HalfToEven")))))))

(fn `UserConstructionScript`)