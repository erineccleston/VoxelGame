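; VoxelBase_BP is a voxel block actor with health that can spawn neighbouring blocks toward a player.
; Damage lowers health, shown live on a text render, and destroys the block at zero.
; Activate rounds the direction to the player into 100-unit Z or Y steps, preferring Z, and line-traces for a free cell before spawning the given class.
; Damage also computes a shrinking DesiredScale, but the cube interpolation that uses it is disconnected.
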(event `self.ReceiveBeginPlay`
  (set `self.CurrentHealth` (`self.MaxHealth`)))

(event `Destroy`
  (`self.K2_DestroyActor`))

(event `self.ReceiveAnyDamage`
  (params (Damage :type "Float (single-precision)") (DamageType :type "DamageType Object Reference") (InstigatedBy :type "Controller Object Reference") (DamageCauser :type "Actor Object Reference"))
  (bind _returnvalue (+ 0.5 (/ (/ (`self.CurrentHealth`) (`self.MaxHealth`)) 2.0)))
  (bind _output_get (set `self.CurrentHealth` (- (`self.CurrentHealth`) Damage)))
  (set `self.DesiredScale` (`KismetMathLibrary.MakeVector` _returnvalue _returnvalue _returnvalue))
  (if (<= _output_get 0.0)
    (`self.Destroy`)))

(event `self.ReceiveTick`
  (params (DeltaSeconds :type "Float (single-precision)"))
  (`TextRenderComponent.K2_SetText` (`self.TextRender`) (`KismetTextLibrary.Conv_DoubleToText` (`self.CurrentHealth`) "HalfToEven")))

(event `Activate`
  (params (Player :type "/Game/Player/Drone_BP Object Reference") (SpawnType :type "/Game/Blueprints/Voxels/VoxelBase_BP Class Reference"))
  (bind _returnvalue (`self.K2_GetActorLocation`))
  (bind (_returnvalue_x _returnvalue_y _returnvalue_z) (`KismetMathLibrary.BreakVector` (`KismetMathLibrary.GetDirectionUnitVector` (`self.K2_GetActorLocation`) (`self.K2_GetActorLocation` Player))))
  (bind _returnvalue_2 (`KismetMathLibrary.MakeVector` 0.0 0.0 (* (`KismetMathLibrary.Round` _returnvalue_z) 100.0)))
  (bind _returnvalue_3 (!= _returnvalue_2 (0.0 0.0 0.0)))
  (bind _returnvalue_4 (+ _returnvalue_2 _returnvalue))
  (bind _returnvalue_5 (+ (`KismetMathLibrary.MakeVector` 0.0 (* (`KismetMathLibrary.Round` _returnvalue_y) 100.0)) _returnvalue))
  (bind _returnvalue_6 (select `bool` _returnvalue_3 :`false` _returnvalue_4 :`true` _returnvalue_5))
  (bind _returnvalue_7 (select `bool` _returnvalue_3 :`false` _returnvalue_5 :`true` _returnvalue_4))
  (if (`KismetSystemLibrary.IsValidClass` SpawnType)
    (bind (_outhit _returnvalue_8) (`KismetSystemLibrary.LineTraceSingle` (`self.K2_GetActorLocation`) _returnvalue_7 "TraceTypeQuery1"))
    (if (not _returnvalue_8)
      (`|SpawnActorFromClass` SpawnType (`KismetMathLibrary.MakeTransform` _returnvalue_7) "AlwaysSpawn" "OverrideRootScale")
      (else
        (bind (_outhit_2 _returnvalue_9) (`KismetSystemLibrary.LineTraceSingle` (`self.K2_GetActorLocation`) _returnvalue_6 "TraceTypeQuery1"))
        (if (and (not _returnvalue_9) (!= _returnvalue_6 (`self.K2_GetActorLocation`)))
          (`|SpawnActorFromClass` SpawnType (`KismetMathLibrary.MakeTransform` _returnvalue_6) "AlwaysSpawn" "OverrideRootScale"))))))

(fn `UserConstructionScript`)