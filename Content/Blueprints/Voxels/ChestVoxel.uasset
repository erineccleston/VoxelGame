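; Chest voxel that gives players a storage inventory they can open in the world.
; Activate finds the first top-level InventoryWidget and shows the player's inventory on the left and the chest's on the right.
; On destruction it calls Empty on its inventory, then runs the parent's Destroyed logic.
; An unconnected loop that spawns a ResourceDrop per filled slot remains in the graph but never runs.
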(event `self.Activate`
  (params (Player :type "/Game/Player/Drone_BP Object Reference") (SpawnType :type "/Game/Blueprints/Voxels/VoxelBase_BP Class Reference"))
  (bind _foundwidgets (`WidgetBlueprintLibrary.GetAllWidgetsOfClass` "/Game/UI/InventoryWidget.InventoryWidget_C"))
  (`/Game/UI/InventoryWidget.Show` (`|GetArrayItem` _foundwidgets) Player (`/Game/Player/Drone_BP.Inventory` Player) (`self.Inventory`)))

(event `self.ReceiveDestroyed`
  (`/Game/Blueprints/InventoryComponent.Empty` (`self.Inventory`) true)
  (`parent.ReceiveDestroyed`))

(fn `UserConstructionScript`
  (`parent.UserConstructionScript`))