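; Indestructible charging-station voxel that recharges the player's drone while it stays in range.
; Box overlap tracks the drone, and Activate opens the InventoryWidget on its inventory and starts charging.
; Tick charges by applying negative damage scaled by ChargeRate and frame time until the drone leaves the box.
; An unused, disconnected branch would move the drone above the block.
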(event `self.ReceiveTick`
  (params (DeltaSeconds :type "Float (single-precision)"))
  (`parent.ReceiveTick` DeltaSeconds)
  (if (`self.DoCharge`)
    (`GameplayStatics.ApplyDamage` (`self.PlayerRef`) (* DeltaSeconds (`self.ChargeRate`) -1.0))))

(event `self.ReceiveAnyDamage`
  (params (Damage :type "Float (single-precision)") (DamageType :type "DamageType Object Reference") (InstigatedBy :type "Controller Object Reference") (DamageCauser :type "Actor Object Reference")))

(event `self.Activate`
  (params (Player :type "/Game/Player/Drone_BP Object Reference") (SpawnType :type "/Game/Blueprints/Voxels/VoxelBase_BP Class Reference"))
  (bind _playerref (`self.PlayerRef`))
  (bind _inventory (`/Game/Player/Drone_BP.Inventory` _playerref))
  (`/Engine/EditorBlueprintResources/StandardMacros.IsValid` _playerref
    (:`Is Valid`
      (bind _foundwidgets (`WidgetBlueprintLibrary.GetAllWidgetsOfClass` "/Game/UI/InventoryWidget.InventoryWidget_C"))
      (`/Game/UI/InventoryWidget.Show` (`|GetArrayItem` _foundwidgets) _playerref _inventory _inventory)
      (set `self.DoCharge` true))))

(event `self.Box.OnComponentEndOverlap`
  (params (OverlappedComponent :type "PrimitiveComponent Object Reference") (OtherActor :type "Actor Object Reference") (OtherComp :type "PrimitiveComponent Object Reference") (OtherBodyIndex :type Integer))
  (cast `/Game/Player/Drone_BP` OtherActor)
  (set `self.PlayerRef` null)
  (set `self.DoCharge` false))

(event `self.Box.OnComponentBeginOverlap`
  (params (OverlappedComponent :type "PrimitiveComponent Object Reference") (OtherActor :type "Actor Object Reference") (OtherComp :type "PrimitiveComponent Object Reference") (OtherBodyIndex :type Integer) (bFromSweep :type Boolean) (SweepResult :type "HitResult Structure (by ref)"))
  (bind _asdrone_bp (cast `/Game/Player/Drone_BP` OtherActor))
  (set `self.PlayerRef` _asdrone_bp))

(fn `UserConstructionScript`
  (`parent.UserConstructionScript`))