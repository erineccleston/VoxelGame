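; Player drone pawn that moves in grid steps, mines and activates voxels under the cursor, and collects resource drops into an inventory.
; Directional inputs queue trace-checked waypoints, merging straight runs, which Tick follows at motor speed.
; Mining and interaction require standing still, range and line of sight traced to target edges and corners, with tool stats from a data table.
; Tick also drives velocity-based tilt and wobble, mouse-parallax camera rotation and smoothed zoom.
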(event `self.ReceiveBeginPlay`
  (set `self.DesiredZoom` (`SpringArmComponent.TargetArmLength` (`self.SpringArm`)))
  (set `PlayerController.bShowMouseCursor` true (cast `PlayerController` (`self.GetController`) :!pure true))
  (`self.SetMiningTool` "Better"))

(event `self.ReceiveTick`
  (params (DeltaSeconds :type "Float (single-precision)"))
  (bind _springarm (`self.SpringArm`))
  (`self.CalcVelocity`)
  (`SceneComponent.K2_SetRelativeRotation` (`self.Body`) (`self.CalcPseduoAnim`) false false)
  (`SceneComponent.K2_SetRelativeRotation` (`self.SpringArm`) (`self.CalcParallax`) false false)
  (set `SpringArmComponent.TargetArmLength` (`KismetMathLibrary.FInterpTo` (`SpringArmComponent.TargetArmLength` _springarm) (`self.DesiredZoom`) (`GameplayStatics.GetWorldDeltaSeconds`) 5.0) _springarm)
  (`self.Move`))

(event `InputAxis|Mine`
  (params (AxisValue :type "Float (single-precision)"))
  (bind (_miningtool_range _miningtool_dps) (break `/Game/Blueprints/Structs/MiningTool` (`self.MiningTool`)))
  ;[1 1 1] Controls
  (if (and (!= AxisValue 0.0) (== (`self.Velocity`) (0.0 0.0 0.0)))
    (bind _actor (`self.GetActorInRange` (+ _miningtool_range 1)))
    (`/Engine/EditorBlueprintResources/StandardMacros.IsValid` _actor
      (:`Is Valid`
        (`GameplayStatics.ApplyDamage` _actor (* _miningtool_dps (`GameplayStatics.GetWorldDeltaSeconds`)))))))

(event `InputAction|Interact`
  (params (Key :type "Key Structure" :default "AnyKey"))
  ;[1 1 1] Controls
  (:`Pressed`
    (if (== (`self.Velocity`) (0.0 0.0 0.0))
      (bind _actor (`self.GetActorInRange` 5))
      (bind _asvoxel_base_bp (cast `/Game/Blueprints/Voxels/VoxelBase_BP` _actor))
      (`/Game/Blueprints/Voxels/VoxelBase_BP.Activate` _asvoxel_base_bp self "/Game/Blueprints/Voxels/VoxelBase_BP.VoxelBase_BP_C"))))

(event `InputAction|MoveUp`
  (params (Key :type "Key Structure" :default "AnyKey"))
  ;[1 1 1] Controls
  (:`Pressed`
    (`self.QueueDirection` (* (`self.GetActorUpVector`) (`self.MovementStep`)))))

(event `InputAction|ZoomIn`
  (params (Key :type "Key Structure" :default "AnyKey"))
  ;[1 1 1] Controls
  (:`Pressed`
    (set `self.DesiredZoom` (`KismetMathLibrary.FClamp` (- (`self.DesiredZoom`) (`self.ZoomStep`)) 140.0 2500.0))))

(event `InputAction|MoveDown`
  (params (Key :type "Key Structure" :default "AnyKey"))
  ;[1 1 1] Controls
  (:`Pressed`
    (`self.QueueDirection` (* (`self.GetActorUpVector`) (* (`self.MovementStep`) -1.0)))))

(event `InputAction|MoveLeft`
  (params (Key :type "Key Structure" :default "AnyKey"))
  ;[1 1 1] Controls
  (:`Pressed`
    (`self.QueueDirection` (* (`self.GetActorRightVector`) (* (`self.MovementStep`) -1.0)))))

(event `InputAction|MoveRight`
  (params (Key :type "Key Structure" :default "AnyKey"))
  ;[1 1 1] Controls
  (:`Pressed`
    (`self.QueueDirection` (* (`self.GetActorRightVector`) (`self.MovementStep`)))))

(event `InputAction|ZoomOut`
  (params (Key :type "Key Structure" :default "AnyKey"))
  ;[1 1 1] Controls
  (:`Pressed`
    (set `self.DesiredZoom` (`KismetMathLibrary.FClamp` (+ (`self.DesiredZoom`) (`self.ZoomStep`)) 140.0 2500.0))))

(event `self.Bounds.OnComponentBeginOverlap`
  (params (OverlappedComponent :type "PrimitiveComponent Object Reference") (OtherActor :type "Actor Object Reference") (OtherComp :type "PrimitiveComponent Object Reference") (OtherBodyIndex :type Integer) (bFromSweep :type Boolean) (SweepResult :type "HitResult Structure (by ref)"))
  (bind _asresource_drop (cast `/Game/Blueprints/ResourceDrop` OtherActor))
  (bind _success (`/Game/Blueprints/InventoryComponent.Add` (`self.Inventory`) (`/Game/Blueprints/ResourceDrop.Type` _asresource_drop)))
  (if _success
    (`self.K2_DestroyActor` _asresource_drop)))

(event `SetMiningTool`
  (params (Name :type Name))
  (bind _returnvalue (`|GetDataTableRow` "/Game/Blueprints/DataTables/ToolTable.ToolTable" Name)
    (:`then`
      (set `self.MiningTool` _returnvalue))
    (:`RowNotFound`
      (`KismetSystemLibrary.PrintString` "Mining tool name not found." true true (struct :`R` 1.0 :`A` 1.0)))))

(fn `CalcParallax`
  (returns (ReturnValue :type "Rotator Structure"))
  (bind (_returnvalue_x _returnvalue_y) (`KismetMathLibrary.BreakVector2D` (`WidgetLayoutLibrary.GetViewportSize`)))
  (bind (_locationx _locationy) (`PlayerController.GetMousePosition` (cast `PlayerController` (`self.GetController`) :!pure true)))
  (bind (_returnvalue_x_2 _returnvalue_y_2) (`KismetMathLibrary.BreakVector2D` (* (* (- (`KismetMathLibrary.MakeVector2D` (/ _locationx _returnvalue_x) (/ _locationy _returnvalue_y)) 0.5) 2.0) (`self.Parallax`))))
  (return (`KismetMathLibrary.MakeRotator` 0.0 (* _returnvalue_y_2 -1.0) _returnvalue_x_2)))

(fn `CalcPseduoAnim`
  (returns (ReturnValue :type "Rotator Structure"))
  (bind _returnvalue (`KismetSystemLibrary.GetGameTimeInSeconds`))
  (bind _wobble (`self.Wobble`))
  (bind (_returnvalue_x _returnvalue_y) (`KismetMathLibrary.BreakVector` (/ (`self.Velocity`) 20.0)))
  (return (`KismetMathLibrary.RInterpTo` (`SceneComponent.RelativeRotation` (`self.Body`)) (`KismetMathLibrary.ComposeRotators` (`KismetMathLibrary.MakeRotator` (* (`KismetMathLibrary.Sin` _returnvalue) _wobble) (* (`KismetMathLibrary.Cos` _returnvalue) _wobble)) (`KismetMathLibrary.MakeRotator` _returnvalue_y (* _returnvalue_x -1.0))) (`GameplayStatics.GetWorldDeltaSeconds`) 5.0)))

(fn `CalcVelocity`
  (set `self.Velocity` (/ (- (`self.K2_GetActorLocation`) (`self.PreviousLocation`)) (`GameplayStatics.GetWorldDeltaSeconds`)))
  (set `self.PreviousLocation` (`self.K2_GetActorLocation`)))

(fn `GetActorInRange`
  (params (Blocks :type Integer))
  (returns (Actor :type "Actor Object Reference"))
  (locals (HitActor :type "Actor Object Reference"))
  (bind _output_get (set `local.HitActor` (`.HitActor` (`GameplayStatics.BreakHitResult` (`PlayerController.GetHitResultUnderCursorByChannel` (cast `PlayerController` (`self.GetController`) :!pure true) "TraceTypeQuery1" true)))))
  (`/Engine/EditorBlueprintResources/StandardMacros.IsValid` _output_get
    (:`Is Valid`
      (if (< (`KismetMathLibrary.VSize` (- (`self.K2_GetActorLocation`) (`self.K2_GetActorLocation` _output_get))) (* Blocks (`self.MovementStep`)))
        (bind _returnvalue (`self.LineOfSight` _output_get))
        (if _returnvalue
          (return (`local.HitActor`))
          (else
            (return null)))))))

(fn `InLine`
  (params (Vector1 :type "Vector Structure") (Vector2 :type "Vector Structure"))
  (returns (ReturnValue :type Boolean))
  (return (or (== Vector1_Y Vector2_Y) (== Vector1_Z Vector2_Z))))

(fn `LineOfSight`
  (params (HitActor :type "Actor Object Reference"))
  (returns (ReturnValue :type Boolean))
  (bind _returnvalue (`self.K2_GetActorLocation` HitActor))
  (bind _y (.y _returnvalue))
  (bind _z (.z _returnvalue))
  (bind _y_2 (.y _returnvalue))
  (bind _z_2 (.z _returnvalue))
  (bind _returnvalue_2 (/ (`self.MovementStep`) 2.0))
  (bind _returnvalue_3 (/ (`self.MovementStep`) 2.0))
  (bind _y_3 (.y (`self.K2_GetActorLocation` HitActor)))
  (bind _z_3 (.z (`self.K2_GetActorLocation` HitActor)))
  (bind _returnvalue_4 (- _z_3 _returnvalue_3))
  (bind _returnvalue_5 (- _y_3 _returnvalue_3))
  (bind _returnvalue_6 (+ _z_3 _returnvalue_3))
  (bind _returnvalue_7 (+ _y_3 _returnvalue_3))
  (for _array_element (`|MakeArray` (`KismetMathLibrary.MakeVector` 0.0 (+ _y _returnvalue_2) _z_2) (`KismetMathLibrary.MakeVector` 0.0 (- _y _returnvalue_2) _z_2) (`KismetMathLibrary.MakeVector` 0.0 _y_2 (+ _z _returnvalue_2)) (`KismetMathLibrary.MakeVector` 0.0 _y_2 (- _z _returnvalue_2)) (`KismetMathLibrary.MakeVector` 0.0 _returnvalue_7 _returnvalue_6) (`KismetMathLibrary.MakeVector` 0.0 _returnvalue_5 _returnvalue_4) (`KismetMathLibrary.MakeVector` 0.0 _returnvalue_5 _returnvalue_6) (`KismetMathLibrary.MakeVector` 0.0 _returnvalue_7 _returnvalue_4))
    (bind _outhit (`KismetSystemLibrary.LineTraceSingle` (`self.K2_GetActorLocation`) _array_element "TraceTypeQuery1" true))
    (if (== HitActor (`.HitActor` (`GameplayStatics.BreakHitResult` _outhit)))
      (return true)))
  (return false))

(fn `Move`
  (bind _locationqueue (`self.LocationQueue`))
  (bind _motors_speed (break `/Game/Blueprints/Structs/Motors` (`self.Motors`)))
  (`/Game/Blueprints/ObjectMacroLibrary.ValidIndex` 0 (`self.LocationQueue`)
    (:`Valid`
      (`self.K2_SetActorLocation` (`KismetMathLibrary.VInterpTo_Constant` (`self.K2_GetActorLocation`) (`|GetArrayItem` (`self.LocationQueue`)) (`GameplayStatics.GetWorldDeltaSeconds`) _motors_speed))
      (if (== (`|GetArrayItem` _locationqueue) (`self.K2_GetActorLocation`))
        (`KismetArrayLibrary.Array_Remove` _locationqueue)))))

(fn `QueueDirection`
  (params (Vector :type "Vector Structure"))
  (locals (TempLocation :type "Vector Structure"))
  (bind _locationqueue (`self.LocationQueue`))
  (bind _locationqueue_2 (`self.LocationQueue`))
  (bind _locationqueue_3 (`self.LocationQueue`))
  (bind _templocation (`local.TempLocation`))
  (bind _locationqueue_4 (`self.LocationQueue`))
  (bind _returnvalue (`KismetArrayLibrary.Array_LastIndex` _locationqueue))
  (bind _returnvalue_2 (`KismetArrayLibrary.Array_LastIndex` _locationqueue_2))
  (bind _returnvalue_3 (- (`KismetArrayLibrary.Array_LastIndex` _locationqueue_3) 1))
  (bind _returnvalue_4 (select `bool` (`KismetArrayLibrary.Array_IsValidIndex` _locationqueue_2 _returnvalue_2) :`false` (`self.K2_GetActorLocation`) :`true` (`|GetArrayItem` _locationqueue_2 _returnvalue_2)))
  (bind _output_get (set `local.TempLocation` (+ Vector _returnvalue_4)))
  (bind (_outhit _returnvalue_5) (`KismetSystemLibrary.LineTraceSingle` _returnvalue_4 _output_get "TraceTypeQuery1" true))
  (if (not _returnvalue_5)
    (bind _returnvalue_6 (`self.InLine` (`local.TempLocation`) (select `bool` (`KismetArrayLibrary.Array_IsValidIndex` _locationqueue_3 _returnvalue_3) :`false` (`self.K2_GetActorLocation`) :`true` (`|GetArrayItem` _locationqueue_3 _returnvalue_3))))
    (if (and _returnvalue_6 (`KismetArrayLibrary.Array_IsValidIndex` _locationqueue _returnvalue))
      (`KismetArrayLibrary.Array_Set` _locationqueue_4 _returnvalue _templocation)
      (else
        (`KismetArrayLibrary.Array_Add` _locationqueue_4 _templocation)))))

(fn `UserConstructionScript`)