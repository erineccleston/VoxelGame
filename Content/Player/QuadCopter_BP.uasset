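; Player-controlled quadcopter that flies along its own axes, turns in quarter steps and zooms an orthographic camera.
; Axis inputs apply swept world offsets along the actor's forward, right and up vectors, scaled by speed and delta time.
; Turn inputs set a target rotation that a shared Alpha timeline lerps toward, with a flag blocking overlapping turns.
; Zoom inputs step the camera's ortho width within clamped limits.
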(event `InputAction|ZoomOut`
  (params (Key :type "Key Structure" :default "AnyKey"))
  (bind _camera (`self.Camera`))
  ;[1 1 1] Zoom
  (:`Pressed`
    (set `CameraComponent.OrthoWidth` (`KismetMathLibrary.FClamp` (- (`CameraComponent.OrthoWidth` _camera) (`self.ZoomSpeed`)) 175.0 10000.0) _camera)))

(event `InputAction|ZoomIn`
  (params (Key :type "Key Structure" :default "AnyKey"))
  (bind _camera (`self.Camera`))
  ;[1 1 1] Zoom
  (:`Pressed`
    (set `CameraComponent.OrthoWidth` (`KismetMathLibrary.FClamp` (+ (`CameraComponent.OrthoWidth` _camera) (`self.ZoomSpeed`)) 175.0 10000.0) _camera)))

(event `InputAxis|MoveUp`
  (params (AxisValue :type "Float (single-precision)"))
  ;[1 1 1] Movement
  (`self.K2_AddActorWorldOffset` (* (`self.GetActorUpVector`) (* AxisValue (`GameplayStatics.GetWorldDeltaSeconds`) (`self.MovementSpeed`))) true))

(event `InputAxis|MoveRight`
  (params (AxisValue :type "Float (single-precision)"))
  ;[1 1 1] Movement
  (`self.K2_AddActorWorldOffset` (* (`self.GetActorRightVector`) (* AxisValue (`GameplayStatics.GetWorldDeltaSeconds`) (`self.MovementSpeed`))) true))

(event `InputAxis|MoveForward`
  (params (AxisValue :type "Float (single-precision)"))
  ;[1 1 1] Movement
  (`self.K2_AddActorWorldOffset` (* (`self.GetActorForwardVector`) (* AxisValue (`GameplayStatics.GetWorldDeltaSeconds`) (`self.MovementSpeed`))) true))

(event `InputAction|TurnLeft`
  (params (Key :type "Key Structure" :default "AnyKey"))
  ;[1 1 1] Rotation
  (:`Pressed`
    (if (not (`self.CurrentlyTurning`))
      (set `self.CurrentlyTurning` true)
      (set `self.TargetRotation` (`KismetMathLibrary.ComposeRotators` (`self.K2_GetActorRotation`) (struct :`Yaw` -90.0)))
      (bind (_direction _alpha) (`Timeline|Alpha` :!via `PlayFromStart` :!label _label)
        (:`Update`
          (`self.K2_SetActorRotation` (`KismetMathLibrary.RLerp` (`self.K2_GetActorRotation`) (`self.TargetRotation`) _alpha true)))
        (:`Finished`
          (set `self.CurrentlyTurning` false))))))

(event `InputAction|TurnRight`
  (params (Key :type "Key Structure" :default "AnyKey"))
  ;[1 1 1] Rotation
  (:`Pressed`
    (if (not (`self.CurrentlyTurning`))
      (set `self.CurrentlyTurning` true)
      (set `self.TargetRotation` (`KismetMathLibrary.ComposeRotators` (`self.K2_GetActorRotation`) (struct :`Yaw` 90.0)))
      (goto _label :!via `PlayFromStart`))))

(fn `UserConstructionScript`)