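; Player controller that moves the possessed drone pawn in fixed steps along its up and right axes, with the mouse cursor shown.
; Input presses queue step offsets, while Tick glides the pawn toward DesiredLocation at constant speed.
; A queued step is consumed once its target shares the pawn's Y or Z, preventing diagonal travel, and advances DesiredLocation only if a visibility trace is clear.
; Some disconnected movement logic remains unused.
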(event `self.ReceiveBeginPlay`
  (set `self.bShowMouseCursor` true)
  (set `self.DesiredLocation` (`self.K2_GetActorLocation` (`self.K2_GetPawn`))))

(event `self.ReceiveTick`
  (params (DeltaSeconds :type "Float (single-precision)"))
  (bind _returnvalue (`self.K2_GetPawn`))
  (bind _desiredlocation (`self.DesiredLocation`))
  (bind _returnvalue_2 (+ _desiredlocation (`|GetArrayItem` (`self.LocationQueue`))))
  (`self.K2_SetActorLocation` _returnvalue (`KismetMathLibrary.VInterpTo_Constant` (`self.K2_GetActorLocation` _returnvalue) (`self.DesiredLocation`) DeltaSeconds (`self.Speed`)) false false)
  (`/Game/Blueprints/ObjectMacroLibrary.Occupied` (`self.LocationQueue`)
    (:`Occupied`
      (bind _bool (`self.InLine` _returnvalue_2))
      (if _bool
        (bind (_outhit _returnvalue_3) (`KismetSystemLibrary.LineTraceSingle` _desiredlocation _returnvalue_2 "TraceTypeQuery1" true))
        (if (not _returnvalue_3)
          (set `self.DesiredLocation` (+ (`self.DesiredLocation`) (`|GetArrayItem` (`self.LocationQueue`)))))
        (`KismetArrayLibrary.Array_Remove` (`self.LocationQueue`))))))

(event `InputAction|MoveUp`
  (params (Key :type "Key Structure" :default "AnyKey"))
  (:`Pressed`
    (`KismetArrayLibrary.Array_Add` (`self.LocationQueue`) (* (`self.GetActorUpVector` (`self.K2_GetPawn`)) (`self.MovementStep`)))))

(event `InputAction|MoveDown`
  (params (Key :type "Key Structure" :default "AnyKey"))
  (:`Pressed`
    (`KismetArrayLibrary.Array_Add` (`self.LocationQueue`) (* (`self.GetActorUpVector` (`self.K2_GetPawn`)) (* (`self.MovementStep`) -1.0)))))

(event `InputAction|MoveLeft`
  (params (Key :type "Key Structure" :default "AnyKey"))
  (:`Pressed`
    (`KismetArrayLibrary.Array_Add` (`self.LocationQueue`) (* (`self.GetActorRightVector` (`self.K2_GetPawn`)) (* (`self.MovementStep`) -1.0)))))

(event `InputAction|MoveRight`
  (params (Key :type "Key Structure" :default "AnyKey"))
  (:`Pressed`
    (`KismetArrayLibrary.Array_Add` (`self.LocationQueue`) (* (`self.GetActorRightVector` (`self.K2_GetPawn`)) (`self.MovementStep`)))))

(fn `InLine`
  (params (Vector :type "Vector Structure"))
  (returns (Bool :type Boolean))
  (bind (_returnvalue_x _returnvalue_y _returnvalue_z) (`KismetMathLibrary.BreakVector` (`self.K2_GetActorLocation` (`self.K2_GetPawn`))))
  (return (or (== _returnvalue_y Vector_Y) (== _returnvalue_z Vector_Z))))

(fn `UserConstructionScript`)